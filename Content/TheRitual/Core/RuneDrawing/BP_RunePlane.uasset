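; Rune drawing plane actor that shows the player's drawn strokes and reacts to rune recognition.
; Draw start spawns a Niagara trail attached to the TrailPainter and a looping sound; a break deactivates the trail, while stopping fades the sound and hides the plane.
; Recognition plays success or failure effects via HasRuneBeenTriggered, then after a delay clears all trails, calls TriggerRune and destroys the actor.
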(event `self.OnDrawStart`
  (bind _currentdrawingtrail (`self.CurrentDrawingTrail`))
  (`|ExecutionSequence`
    (:`then_0`
      (bind _returnvalue (`AddComponent|NODE_AddNiagaraComponent-0`))
      (bind _output_get (set `self.CurrentDrawingTrail` _returnvalue))
      (`ActorComponent.Activate` _output_get false)
      (`KismetArrayLibrary.Array_Add` (`self.DrawnTrails`) _currentdrawingtrail)
      (`SceneComponent.K2_AttachToComponent` _currentdrawingtrail (`self.TrailPainter`) "None" "SnapToTarget" "SnapToTarget" "KeepRelative" true))
    (:`then_1`
      (bind _returnvalue_2 (`GameplayStatics.SpawnSound2D` "/Game/TheRitual/Sounds/Samples/Runes/draw_loop.draw_loop" 1.0 1.0 0.0 null)))))

(event `self.OnDrawBreak`
  (`ActorComponent.Deactivate` (`self.CurrentDrawingTrail`)))

(event `self.OnDrawStop`
  (`|ExecutionSequence`
    (:`then_0`
      (`AudioComponent.FadeOut` (stale `self.OnDrawStart` _returnvalue_2) 0.5 0.0 "SCurve"))
    (:`then_1`
      (`SceneComponent.SetVisibility` (`self.RunePlane`) false false))))

(event `self.OnRuneRecognized`
  (params (runeName :type String))
  (bind _returnvalue (`self.HasRuneBeenTriggered` runeName))
  (if _returnvalue
    (`ActorComponent.Activate` (`self.PSN_Success`) false)
    (`GameplayStatics.PlaySound2D` "/Game/TheRitual/Sounds/Samples/Runes/rune_sucess.rune_sucess" 1.0 1.0 0.0 null null)
    (else
      (`ActorComponent.Activate` (`self.PSN_Failed`) false)))
  (`KismetSystemLibrary.Delay` 3.0)
  (for _array_element (`self.DrawnTrails`)
    (`ActorComponent.K2_DestroyComponent` _array_element))
  (`self.TriggerRune`)
  (`self.K2_DestroyActor`))

(fn `UserConstructionScript`)