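; BP_KiYApproaching is a trigger actor running the KiY chase encounter in The Ritual.
; When activated, player overlap reveals KiY and moves it toward ChaseTarget with MoveComponentTo; leaving hides and resets it.
; Tick checks player distance to halt the move, play the attack and, after a delay, teleport the player to PlayerRespawn.
; OnKiYDestruction during a chase stops KiY, sets the AnimBP's Killed flag and opens the Credits level after a delay.
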(event `self.ReceiveBeginPlay`
  ;[1 1 1] Init
  (bind _asabp_tki_y_s4 (cast `/Game/TheRitual/Art/Characters/TKiY_v3/ABP_TKiY_S4` (`SkeletalMeshComponent.GetAnimInstance` (`SkeletalMeshActor.SkeletalMeshComponent` (`self.KiY`)))))
  (set `self.AnimationBlueprint` _asabp_tki_y_s4)
  (set `self.StartPosition` (`SceneComponent.K2_GetComponentLocation` (`AnimInstance.GetOwningComponent` (`self.AnimationBlueprint`))))
  (`SceneComponent.SetVisibility` (`AnimInstance.GetOwningComponent` (`self.AnimationBlueprint`)) false false))

(event `self.ReceiveTick`
  (params (DeltaSeconds :type "Float (single-precision)"))
  (if (`self.Active`)
    (if (< (`KismetMathLibrary.Vector_Distance` (`self.K2_GetActorLocation` (`self.KiY`)) (`self.K2_GetActorLocation` (`GameplayStatics.GetPlayerPawn` 0))) (`self.MaxDistance`))
      ;[1 1 1] Attack
      (`|ExecutionSequence`
        (:`then_0`
          (set `/Game/TheRitual/Art/Characters/TKiY_v3/ABP_TKiY_S4.Attack` true (`self.AnimationBlueprint`))
          (`KismetSystemLibrary.Delay` (`self.AttackDuration`))
          (`self.K2_SetActorLocation` (`GameplayStatics.GetPlayerPawn` 0) (`SceneComponent.K2_GetComponentLocation` (`self.PlayerRespawn`)) false false))
        (:`then_1`
          (goto _label :!via `Stop`))))))

(event `self.ReceiveActorBeginOverlap`
  (params (OtherActor :type "Actor Object Reference"))
  (bind _animationblueprint (`self.AnimationBlueprint`))
  ;[1 1 1] Activate and Trigger Chase
  (if (`self.Activated`)
    (set `self.Active` true)
    (`SceneComponent.SetVisibility` (`AnimInstance.GetOwningComponent` (`self.AnimationBlueprint`)) true false)
    (set `/Game/TheRitual/Art/Characters/TKiY_v3/ABP_TKiY_S4.Attack` false _animationblueprint)
    (set `/Game/TheRitual/Art/Characters/TKiY_v3/ABP_TKiY_S4.Killed` false _animationblueprint)
    (set `/Game/TheRitual/Art/Characters/TKiY_v3/ABP_TKiY_S4.StartSequence` true _animationblueprint)
    (`KismetSystemLibrary.MoveComponentTo` (`Actor.RootComponent` (`self.KiY`)) (`SceneComponent.K2_GetComponentLocation` (`self.ChaseTarget`)) (struct :`Yaw` -90.0) false false (`self.Speed`) :!label _label)))

(event `self.ReceiveActorEndOverlap`
  (params (OtherActor :type "Actor Object Reference"))
  ;[1 1 1] Stop Chase and Reset
  (set `self.Active` false)
  (`SceneComponent.SetVisibility` (`Actor.RootComponent` (`self.KiY`)) false false)
  (`SceneComponent.K2_SetWorldLocation` (`Actor.RootComponent` (`self.KiY`)) (`self.StartPosition`) false false)
  (goto _label :!via `Stop`))

(event `OnKiYDestruction`
  ;[1 1 1] Die and go to Credits
  (if (`self.Active`)
    (`|ExecutionSequence`
      (:`then_0`
        (goto _label :!via `Stop`))
      (:`then_1`
        (set `self.Active` false)
        (set `/Game/TheRitual/Art/Characters/TKiY_v3/ABP_TKiY_S4.Killed` true (`self.AnimationBlueprint`))
        (`KismetSystemLibrary.Delay` (`self.DieDuration`))
        (`GameplayStatics.OpenLevelBySoftObjectPtr` "/Game/TheRitual/Maps/Credits.Credits")))))

(fn `UserConstructionScript`)