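; A VR pickup actor that triggers a rune when grabbed through BP_MotionController.
; Pickup disables physics, attaches the actor to the given component, calls EnableRune and has BP_CharacterController show the rune effect matching RuneName on the hand.
; It also plays a pickup sound, plus a 2D sound on the first grab only.
; Drop restores physics, detaches the actor and plays a drop sound.
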(event `/Game/VirtualRealityBP/Blueprints/PickupActorInterface.Pickup`
  (params (AttachTo :type "SceneComponent Object Reference"))
  ;[1 1 1] Pick Up
  (`|ExecutionSequence`
    (:`then_0`
      (`PrimitiveComponent.SetSimulatePhysics` (`self.StaticMeshComponent`) false)
      (`SceneComponent.K2_AttachToComponent` (`self.K2_GetRootComponent`) AttachTo "None" "KeepWorld" "KeepWorld" "KeepWorld" false)
      (`self.EnableRune`)
      ;[1 1 1] Trigger rune effect on hand
      (bind _asbp_character_controller (cast `/Game/TheRitual/Core/PlayerController/BP_CharacterController` (`GameplayStatics.GetPlayerCharacter` 0)))
      (switch `string` (`self.RuneName`)
        (:`Z`
          (`/Game/TheRitual/Core/PlayerController/BP_CharacterController.ShowRune` _asbp_character_controller "NewEnumerator0"))
        (:`Light`
          (`/Game/TheRitual/Core/PlayerController/BP_CharacterController.ShowRune` _asbp_character_controller "NewEnumerator1"))
        (:`Reconstruction`
          (`/Game/TheRitual/Core/PlayerController/BP_CharacterController.ShowRune` _asbp_character_controller "NewEnumerator2"))
        (:`Destruction`
          (`/Game/TheRitual/Core/PlayerController/BP_CharacterController.ShowRune` _asbp_character_controller "NewEnumerator3"))))
    (:`then_1`
      (`GameplayStatics.PlaySoundAtLocation` (`self.Sound_up`) (`self.K2_GetActorLocation`) (struct) 1.0 1.0 0.0 null null null)
      (`/Engine/EditorBlueprintResources/StandardMacros.DoOnce` false
        (:`Completed`
          (`GameplayStatics.PlaySound2D` (`self.sound_once`) 1.0 1.0 0.0 null null))))))

(event `/Game/VirtualRealityBP/Blueprints/PickupActorInterface.Drop`
  ;[1 1 1] Let go
  (`PrimitiveComponent.SetSimulatePhysics` (`self.StaticMeshComponent`) true)
  (`self.K2_DetachFromActor` "KeepWorld" "KeepWorld" "KeepWorld")
  (`GameplayStatics.PlaySoundAtLocation` (`self.Sound_down`) (`self.K2_GetActorLocation`) (struct) 1.0 1.0 0.0 null null null))

(fn `UserConstructionScript`)