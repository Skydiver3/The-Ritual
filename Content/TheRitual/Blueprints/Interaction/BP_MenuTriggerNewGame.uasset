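; A menu trigger actor that starts a new game when a motion controller overlaps it.
; On BeginPlay it hides its sprite component.
; On overlap with a BP_MotionController it waits briefly, hides the rune circle and activates a success particle effect, then after a second delay opens the PhoneRoom level.
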(event `self.ReceiveBeginPlay`
  (`SceneComponent.SetVisibility` (`self.SpriteComponent`) false false))

(event `self.ReceiveActorBeginOverlap`
  (params (OtherActor :type "Actor Object Reference"))
  (if (== (`GameplayStatics.GetObjectClass` OtherActor) "/Game/VirtualRealityBP/Blueprints/BP_MotionController.BP_MotionController_C")
    (`KismetSystemLibrary.Delay` 1.0)
    (`SceneComponent.SetVisibility` (`self.RuneCircle`) false false)
    (`ActorComponent.Activate` (`self.PSN_Success`) false)
    (`KismetSystemLibrary.Delay` 2.0)
    (`GameplayStatics.OpenLevelBySoftObjectPtr` "/Game/TheRitual/Maps/PhoneRoom.PhoneRoom")))

(fn `UserConstructionScript`)