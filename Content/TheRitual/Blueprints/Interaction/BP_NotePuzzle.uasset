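; BP_NotePuzzle is an interaction Blueprint that activates a linked KiYTrigger and shows a rune through the player character.
; Its ActivateKiYTrigger event sets the trigger's Activated flag, then switches on EnabledRuneName to pass the matching rune to BP_CharacterController's ShowRune.
; The Triggered guard is only ever set to false here, so this event never latches itself against repeat activation.
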(event `self.ActivateKiYTrigger`
  (if (not (`self.Triggered`))
    (set `self.Triggered` false)
    (set `/Game/TheRitual/Blueprints/Interaction/BP_KiYApproaching.Activated` true (`self.KiYTrigger`))
    (bind _asbp_character_controller (cast `/Game/TheRitual/Core/PlayerController/BP_CharacterController` (`GameplayStatics.GetPlayerCharacter` 0)))
    (switch `string` (`self.EnabledRuneName`)
      (:`Z`
        (`/Game/TheRitual/Core/PlayerController/BP_CharacterController.ShowRune` _asbp_character_controller "NewEnumerator0"))
      (:`Light`
        (`/Game/TheRitual/Core/PlayerController/BP_CharacterController.ShowRune` _asbp_character_controller "NewEnumerator1"))
      (:`Reconstruction`
        (`/Game/TheRitual/Core/PlayerController/BP_CharacterController.ShowRune` _asbp_character_controller "NewEnumerator2"))
      (:`Destruction`
        (`/Game/TheRitual/Core/PlayerController/BP_CharacterController.ShowRune` _asbp_character_controller "NewEnumerator3")))))

(fn `UserConstructionScript`)