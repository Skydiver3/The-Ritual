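; BP_Madness is an actor that toggles a madness effect in the game through TriggerMadness and RemoveMadness events.
; These show or hide the MadnessActors, switch a Material Parameter Collection scalar between AnimShadowMax and zero, and fade an audio component in or out.
; While madness is active, a gate lets Tick feed the distance between KiY and this actor into an audio float parameter.
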(event `self.ReceiveBeginPlay`
  (`|ExecutionSequence`
    (:`then_0`
      (bind _returnvalue (`AddComponent|NODE_AddAudioComponent-0`))
      (set `self.AudioComp` _returnvalue))
    (:`then_1`
      (`AudioComponent.FadeOut` (`self.AudioComp`) 0.0 0.0 "SCurve"))))

(event `TriggerMadness`
  (`|ExecutionSequence`
    (:`then_0`
      (for _array_element (`self.MadnessActors`)
        (`self.SetActorHiddenInGame` _array_element false)
        (`KismetMaterialLibrary.SetScalarParameterValue` (`self.MPC`) (`self.Name`) (`self.AnimShadowMax`))))
    (:`then_1`
      (`AudioComponent.FadeIn` (`self.AudioComp`) 1.2 1.0 0.0 "Logarithmic"))
    (:`then_2`
      (goto _label :!via `Open`))))

(event `RemoveMadness`
  (`|ExecutionSequence`
    (:`then_0`
      (for _array_element (`self.MadnessActors`)
        (`self.SetActorHiddenInGame` _array_element true)
        (`KismetMaterialLibrary.SetScalarParameterValue` (`self.MPC`) (`self.Name`))))
    (:`then_1`
      (`AudioComponent.FadeOut` (`self.AudioComp`) 0.8 0.0 "SCurve"))
    (:`then_2`
      (goto _label :!via `Close`))))

(event `self.ReceiveTick`
  (params (DeltaSeconds :type "Float (single-precision)"))
  (`/Engine/EditorBlueprintResources/StandardMacros.Gate` true :!label _label
    (:`Exit`
      (`AudioComponent.SetFloatParameter` (`self.AudioComp`) "DIstance to KiY" (`KismetMathLibrary.Vector_Distance` (`self.K2_GetActorLocation` (`self.KiY`)) (`self.K2_GetActorLocation`))))))

(fn `UserConstructionScript`)