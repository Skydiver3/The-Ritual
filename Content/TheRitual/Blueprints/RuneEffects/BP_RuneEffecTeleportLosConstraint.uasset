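; Rune effect Blueprint for a teleport (line-of-sight constrained, by its name) that adds visual feedback around the effect.
; On recognition it waits briefly, then plays the pre-teleport effect at the player's position; the trigger event calls ExecuteEffect.
; On execution it plays the post-teleport effect and, if not yet Triggered, briefly shows an animated skeletal mesh (tentacles), optionally destroying itself afterwards.
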(event `self.OnEffectRecognized`
  ;[1 1 1] Pre-teleport effect
  (`KismetSystemLibrary.Delay` 1.0)
  (bind _returnvalue (`self.GetPlayerPosition`))
  (`SceneComponent.K2_SetWorldLocation` (`self.Pre_teleport`) _returnvalue false false)
  (`ActorComponent.Activate` (`self.Pre_teleport`) false))

(event `self.OnEffectTriggered`
  (`self.ExecuteEffect`))

(event `self.OnEffectExecuted`
  (bind _returnvalue (`self.GetComponentByClass` (`self.SkeletalMeshActor`) "/Script/Engine.SkeletalMeshComponent"))
  ;[1 1 1] Post-teleport effect
  (`ActorComponent.Activate` (`self.Post_teleport`) false)
  ;[1 1 1] Play Animation (for Tentacles) on first time teleport
  (if (!= (`self.SkeletalMeshActor`) null)
    (if (not (`self.triggered`))
      (`SceneComponent.SetVisibility` _returnvalue true false)
      (`SkeletalMeshComponent.Play` _returnvalue false)
      (`KismetSystemLibrary.Delay` (`self.AnimationDuration`))
      (`SceneComponent.SetVisibility` _returnvalue false false)
      (if (`self.destroyAfterPlay`)
        (`self.K2_DestroyActor`)))))

(fn `UserConstructionScript`)