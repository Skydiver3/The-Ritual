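; Rune effect Blueprint that temporarily shows a referenced skeletal mesh actor and plays its animation when the effect triggers.
; OnEffectTrigger makes the actor's skeletal mesh component visible, plays it without looping, then hides it after a Delay of AnimationDuration.
; The hide relies on that timer alone, not on an animation-finished callback.
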(event `self.OnEffectTrigger`
  (bind _returnvalue (`self.GetComponentByClass` (`self.SkeletalMeshActor`) "/Script/Engine.SkeletalMeshComponent"))
  (`SceneComponent.SetVisibility` _returnvalue true false)
  (`SkeletalMeshComponent.Play` _returnvalue false)
  (`KismetSystemLibrary.Delay` (`self.AnimationDuration`))
  (`SceneComponent.SetVisibility` _returnvalue false false))

(fn `UserConstructionScript`
  (`parent.UserConstructionScript`))