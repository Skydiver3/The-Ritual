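; Rune effect that plays a reassembly animation, apparently repairing stairs, when triggered while a constraint actor passes an angle-based line-of-sight check.
; On trigger it toggles the start show/hide lists, plays the skeletal mesh animation and a 2D "getting back together" sound.
; After the animation duration it reveals finish actors (hidden at BeginPlay), moves the fixed stairs into position inside that loop, and destroys the hide-on-finish actors.
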(event `self.ReceiveBeginPlay`
  (`parent.ReceiveBeginPlay`)
  (for _array_element (`self.ShowOnFinish`)
    (`SceneComponent.SetVisibility` (`Actor.RootComponent` _array_element) false false)))

(event `self.OnEffectTrigger`
  (bind _returnvalue (`self.IsInLineOfSight` (`self.LoSConstraint`) (`self.MinAngle`)))
  (if _returnvalue
    (`|ExecutionSequence`
      (:`then_0`
        (for _array_element (`self.ShowOnStart`)
          (`SceneComponent.SetVisibility` (`Actor.RootComponent` _array_element) true false))
        (for _array_element_2 (`self.HideOnStart`)
          (`SceneComponent.SetVisibility` (`Actor.RootComponent` _array_element_2) false false))
        (`SkeletalMeshComponent.Play` (`self.GetComponentByClass` (`self.SkeletalMeshActor`) "/Script/Engine.SkeletalMeshComponent") false)
        (`KismetSystemLibrary.Delay` (`self.AnimationDuration`))
        (for _array_element_3 (`self.ShowOnFinish`)
          (`SceneComponent.SetVisibility` (`Actor.RootComponent` _array_element_3) true false)
          (`self.K2_SetActorLocation` (`self.StairsFixed`) (`SceneComponent.K2_GetComponentLocation` (`self.Stairs pos`)) false false))
        (for _array_element_4 (`self.HideOnFinish`)
          (`self.K2_DestroyActor` _array_element_4)))
      (:`then_1`
        (`GameplayStatics.PlaySound2D` "/Game/TheRitual/Sounds/Samples/other/object_getting_back_together_5s.object_getting_back_together_5s" 1.0 1.0 0.0 null null)))))

(fn `UserConstructionScript`
  (`parent.UserConstructionScript`))