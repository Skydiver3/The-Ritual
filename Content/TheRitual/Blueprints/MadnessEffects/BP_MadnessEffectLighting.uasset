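; Madness effect that switches the world between normal and Carcosa lighting when madness starts or stops.
; A dynamic post-process material added to the volume gets its two reach parameters driven by start and end blend timelines, bracketing the streaming-level swaps.
; Between blends, further timelines animate glowing-goo disintegration around loading or unloading the madness objects.
; Start and stop share one timeline chain, branched by a flag, which also fades moving shadows through a parameter collection.
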(event `BlendLighting`
  (params (Time :type "Float (double-precision)"))
  (bind _reach (`self.Reach`))
  (bind _mid (`self.MID`))
  (if (`self.TransitionFinished`)
    (`MaterialInstanceDynamic.SetScalarParameterValue` (`self.MID`) "ReachFirst" (* Time _reach))
    (else
      (`MaterialInstanceDynamic.SetScalarParameterValue` _mid "ReachSecond" (* _reach Time))
      (`MaterialInstanceDynamic.K2_GetScalarParameterValue` _mid "ReachSecond"))))

(event `self.ReceiveBeginPlay`
  (bind _mid (`self.MID`))
  (bind _settings (`PostProcessVolume.Settings` (`self.PostProcessVolume`)))
  (`parent.ReceiveBeginPlay`)
  (bind _returnvalue (`KismetMaterialLibrary.CreateDynamicMaterialInstance` "/Game/TheRitual/Art/PostProcessing/PP_LightChange.PP_LightChange"))
  (set `self.MID` _returnvalue)
  (bind _output_get (set `self.PostProcessMaterials` (`.Array` (break `WeightedBlendables` (`.WeightedBlendables` (break `PostProcessSettings` _settings))))))
  (`KismetArrayLibrary.Array_Add` _output_get (make `WeightedBlendable` 1.0 (`self.MID`)))
  (bind _structout (setmembers `PostProcessSettings` :`StructRef` _settings :`WeightedBlendables` (make `WeightedBlendables` (`self.PostProcessMaterials`))))
  (set `PostProcessVolume.Settings` _structout (`self.PostProcessVolume`))
  (`MaterialInstanceDynamic.SetScalarParameterValue` _mid "ReachFirst" 0.0)
  (`MaterialInstanceDynamic.SetScalarParameterValue` _mid "ReachSecond" 0.0)
  (`MaterialInstanceDynamic.SetScalarParameterValue` _mid "TransitionFogStart" (`self.FogStart`))
  (`MaterialInstanceDynamic.SetScalarParameterValue` _mid "FogTransition" (`self.FogTransition`))
  (`KismetMaterialLibrary.SetScalarParameterValue` "/Game/TheRitual/Art/Effects/GlowingGoo/MPC_GlowingGoo.MPC_GlowingGoo" "Disintegration" 1.0))

(event `self.OnMadnessStart`
  (bind _mid (`self.MID`))
  (set `self.TriggeredMadnessStart` true)
  (set `self.MadnessIsEnding` false)
  (set `self.TransitionFinished` false)
  (bind (_direction _time) (`Timeline|StartBlendTimeline` :!via `PlayFromStart` :!label _label)
    (:`Update`
      (`self.BlendLighting` _time)
      (`KismetMaterialLibrary.SetScalarParameterValue` "/Game/TheRitual/Art/Environment/MasterMaterials/MPC_OpaqueMaster.MPC_OpaqueMaster" "AnimShadows" (`KismetMathLibrary.Lerp` (* _time (`self.MovingShadowsOpacity`)) (* (- 1.0 _time) (`self.MovingShadowsOpacity`)) (`KismetMathLibrary.Conv_BoolToDouble` (`self.MadnessIsEnding`)))))
    (:`Finished`
      (if (`self.MadnessIsEnding`)
        (bind (_direction_2 _newtrack_0) (`Timeline|Timeline_0` :!via `PlayFromStart`)
          (:`Update`
            (`KismetMaterialLibrary.SetScalarParameterValue` "/Game/TheRitual/Art/Effects/GlowingGoo/MPC_GlowingGoo.MPC_GlowingGoo" "Disintegration" _newtrack_0))
          (:`Finished`
            (`GameplayStatics.UnloadStreamLevel` "MadnessObjects")
            (`GameplayStatics.UnloadStreamLevel` "CarcosaLighting")
            (`GameplayStatics.LoadStreamLevel` "NormalLighting" true)
            (set `self.TransitionFinished` true :!label _label_2)
            (bind (_direction_3 _time_2) (`Timeline|EndBlendTimeline` :!via `PlayFromStart`)
              (:`Update`
                (`self.BlendLighting` _time_2))
              (:`Finished`
                (`MaterialInstanceDynamic.SetScalarParameterValue` _mid "ReachFirst" 0.0)
                (`MaterialInstanceDynamic.SetScalarParameterValue` _mid "ReachSecond" 0.0)))))
        (else
          (`GameplayStatics.UnloadStreamLevel` "NormalLighting")
          (`KismetMaterialLibrary.SetScalarParameterValue` "/Game/TheRitual/Art/Effects/GlowingGoo/MPC_GlowingGoo.MPC_GlowingGoo" "Disintegration" 1.0)
          (`GameplayStatics.LoadStreamLevel` "MadnessObjects" true)
          (bind (_direction_4 _newtrack_0_2) (`Timeline|Timeline_1` :!via `PlayFromStart`)
            (:`Update`
              (`KismetMaterialLibrary.SetScalarParameterValue` "/Game/TheRitual/Art/Effects/GlowingGoo/MPC_GlowingGoo.MPC_GlowingGoo" "Disintegration" (- 1.0 _newtrack_0_2)))
            (:`Finished`
              (`GameplayStatics.LoadStreamLevel` "CarcosaLighting" true)
              (goto _label_2))))))))

(event `self.OnMadnessStop`
  (set `self.MadnessIsEnding` true)
  (set `self.TransitionFinished` false)
  (goto _label :!via `PlayFromStart`))

(fn `UserConstructionScript`
  (`parent.UserConstructionScript`))